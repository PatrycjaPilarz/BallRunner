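; BP_WinVoliume is a trigger volume that completes the level when the player overlaps it and no Crystal actors remain in the world.
; The overlap event uses Get All Actors Of Class to check for leftover crystals.
; On completion, it looks up the current level name in the ordered LevelNames array, then opens the next entry or quits the game on the final level.
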(event Collision|EventActorBeginOverlap
  (params (OtherActor :type Actor%20Object%20Reference))
  (Utilities|IsPlayer OtherActor
    (:Is%20Player
      (if (not (CallFunction|AnyCrystalsRemaining))
        (Levelmanagment|CompleteLevel)))))

(fn ConstructionScript)

(fn AnyCrystalsRemaining
  (bind _outactors (Actor|GetAllActorsOfClass "/Game/Blueprints/Actors/Collectables/Crystal.Crystal_C"))
  (return (> (Utilities|Array|Length _outactors) 0)))

(fn CompleteLevel
  (if (LevelManagment|IsFInalLevel)
    (Game|QuitGame 0 "Quit")
    (else
      (LevelManagment|LoadNextLevel))))

(fn GetCurrentLevelIndex
  (bind _returnvalue (Game|GetCurrentLevelName true))
  (return (Utilities|Array|FindItem (Variables|Default|GetLevel%20Names) (Utilities|String|StringToName _returnvalue))))

(fn IsFInalLevel
  (return (== (Utilities|Array|LastIndex (Variables|Default|GetLevel%20Names)) (LevelManagment|GetCurrentLevelIndex))))

(fn LoadNextLevel
  (Game|OpenLevel(byName) (CallFunction|GetNextLevelName (Variables|Default|GetLevel%20Names))))

(fn GetNextLevelName
  (params (Array :type Array%20of%20Names))
  (return (Utilities|Array|Get(acopy) Array (+ (LevelManagment|GetCurrentLevelIndex) 1))))